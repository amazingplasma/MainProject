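; BP_Shotgun is a weapon Blueprint that fires a spread of hitscan pellets on the shoot input, rate-limited by a delay.
; Each shot loops object line traces along the bullet path, offsetting each endpoint by random per-axis spread and replaying the first-person rifle montage.
; Traces that hit a BP_Target call its TargetHit.
; Interact and Discardment defer to the parent class.
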(event Input|EnhancedActionEvents|EnhancedInputActionIA_Shoot
  (params (ActionValue :type Boolean) (ElapsedSeconds :type Float%20%28double-precision%29) (TriggeredSeconds :type Float%20%28double-precision%29) (InputAction :type Input%20Action%20Object%20Reference :default "/Game/FirstPerson/Input/Actions/IA_Shoot.IA_Shoot"))
  (CallFunction|AttemptFire)
  (Utilities|FlowControl|Delay (Variables|Default|GetDelay%20Time))
  (Variables|Default|SetCan%20Fire%20Again true))

(event EventDiscardment
  (|CallParentFunction))

(event EventAttemptFire
  (bind (_start_position _end_position) (CallFunction|CalculateBulletStartandEndPosition 1e+04))
  (bind _spread (Variables|Default|GetSpread))
  (bind (_random_spread_x _random_spread_y _random_spread_z) (CallFunction|CalculateRandomSpread _spread))
  ;[0.15 0.15 0.15 0.5] From 3d Tutorial
  (if (Variables|Default|GetCan%20Fire%20Again)
    (Variables|Default|SetCan%20Fire%20Again false)
    (for _index (range 0 8)
      (bind _outhit (Collision|LineTraceForObjects _start_position (+ _start_position (- _end_position _start_position) (Math|Vector|MakeVector _random_spread_x _random_spread_y _random_spread_z)) (Utilities|Array|MakeArray "ObjectTypeQuery1" "ObjectTypeQuery2" "ObjectTypeQuery6") false 0 "ForOneFrame"))
      (Animation|Montage|MontagePlay (Components|SkeletalMesh|GetAnimInstance (Variables|/Game/FirstPerson/Blueprints/BP_FirstPersonCharacter.BP_FirstPersonCharacter_C|GetFirstPersonMesh (Variables|Default|GetPlayer%20Ref))) "/Game/FirstPersonArms/Animations/FP_Rifle_Shoot_Montage.FP_Rifle_Shoot_Montage" 1.0 "MontageLength" 0.0 true)
      (bind _asbp_target (Utilities|Casting|CastToBP_Target (.HitActor (Collision|BreakHitResult _outhit))))
      (Default|TargetHit _asbp_target))))

(event EventInteract
  (params (Player%20Ref :type BP%20First%20Person%20Character%20Object%20Reference))
  ;[0.15 0.15 0.15 0.5] From 3d Tutorial
  (|CallParentFunction Player%20Ref))

(fn ConstructionScript
  (|CallParentFunction))

(fn CalculateRandomSpread
  (params (Spread :type Float%20%28double-precision%29))
  ;[0.15 0.15 0.15 0.5] From 3d Tutorial
  (return (Math|Random|RandomFloatinRange (* Spread -1.0) Spread) (Math|Random|RandomFloatinRange (* Spread -1.0) Spread) (Math|Random|RandomFloatinRange (* Spread -1.0) Spread)))