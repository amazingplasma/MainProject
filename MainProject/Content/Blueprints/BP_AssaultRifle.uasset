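; BP_AssaultRifle is a player weapon that fires three-shot hitscan bursts at targets.
; IA_Shoot starts a burst gated by CanFireAgain, which resets after DelayTime.
; Each shot in BurstFireHelper runs an object line trace, plays the first-person rifle montage and calls TargetHit on any BP_Target hit.
; Interact and Discardment defer to the parent class, while IA_Discard spawns another rifle offset from the player.
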(event Custom|BurstFire
  (if (Variables|Default|GetCan%20Fire%20Again)
    (Variables|Default|SetCan%20Fire%20Again false)
    (CallFunction|BurstFireHelper)
    (Utilities|FlowControl|Delay 0.2)
    (CallFunction|BurstFireHelper)
    (Utilities|FlowControl|Delay 0.2)
    (CallFunction|BurstFireHelper)))

(event Input|EnhancedActionEvents|EnhancedInputActionIA_Shoot
  (params (ActionValue :type Boolean) (ElapsedSeconds :type Float%20%28double-precision%29) (TriggeredSeconds :type Float%20%28double-precision%29) (InputAction :type Input%20Action%20Object%20Reference :default "/Game/FirstPerson/Input/Actions/IA_Shoot.IA_Shoot"))
  (CallFunction|BurstFire)
  (Utilities|FlowControl|Delay (Variables|Default|GetDelay%20Time))
  (Variables|Default|SetCan%20Fire%20Again true))

(event Input|EnhancedActionEvents|EnhancedInputActionIA_Discard
  (params (ActionValue :type Boolean) (ElapsedSeconds :type Float%20%28double-precision%29) (TriggeredSeconds :type Float%20%28double-precision%29) (InputAction :type Input%20Action%20Object%20Reference :default "/Game/Blueprints/IA_Discard.IA_Discard"))
  (bind _player_ref (Variables|Default|GetPlayer%20Ref))
  (bind _returnvalue (Transformation|GetActorTransform _player_ref))
  (Game|SpawnActorfromClass "BP_AssaultRifle_C" (Math|Transform|MakeTransform (+ (.location _returnvalue) "20.000000,0.000000,0.000000") "0, 0, 0" (.scale _returnvalue)) "Undefined" "MultiplyWithRoot" 0 0))

(event EventDiscardment
  (|CallParentFunction))

(event EventInteract
  (params (Player%20Ref :type BP%20First%20Person%20Character%20Object%20Reference))
  (|CallParentFunction Player%20Ref))

(fn ConstructionScript
  (|CallParentFunction))

(fn BurstFireHelper
  (bind (_start_position _end_position) (CallFunction|CalculateBulletStartandEndPosition 1e+03))
  (bind _outhit (Collision|LineTraceForObjects _start_position _end_position (Utilities|Array|MakeArray "ObjectTypeQuery1" "ObjectTypeQuery2" "ObjectTypeQuery6") false 0 "None"))
  (Animation|Montage|MontagePlay (Components|SkeletalMesh|GetAnimInstance (Variables|/Game/FirstPerson/Blueprints/BP_FirstPersonCharacter.BP_FirstPersonCharacter_C|GetFirstPersonMesh (Variables|Default|GetPlayer%20Ref))) "/Game/FirstPersonArms/Animations/FP_Rifle_Shoot_Montage.FP_Rifle_Shoot_Montage" 1.0 "MontageLength" 0.0 true)
  (bind _asbp_target (Utilities|Casting|CastToBP_Target (.HitActor (Collision|BreakHitResult _outhit))))
  (Default|TargetHit _asbp_target))