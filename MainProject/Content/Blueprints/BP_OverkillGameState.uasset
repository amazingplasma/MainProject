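; Game state for Overkill that runs a round-based, timed target-hitting game.
; It counts BP_Target actors to set a countdown, which Tick drains at double speed, showing game over at zero.
; Clearing all targets shows the next-round UI, immediately starts the next round and recounts targets.
; Each clear also spawns a target at the player's starting location, as the lerp toward recorded movement history uses zero alpha.
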(event Custom|Start
  ;[0.15 0.15 0.15 0.5] From 3D Tutorial
  (Variables|Default|SetTimer%20Started? true)
  (Default|PlayerStart (Variables|Default|GetPlayer%20Ref)))

(event Custom|Check%20if%20Game%20Over
  (if (<= (Variables|Default|GetTotal%20Time) 0.0)
    (CallFunction|GameOver)))

(event Custom|Create%20New%20Target
  (bind _player_ref (Variables|Default|GetPlayer%20Ref))
  (bind _player_ref_2 (Variables|Default|GetPlayer%20Ref))
  (bind _player_movement_history (Variables|/Game/FirstPerson/Blueprints/BP_FirstPersonCharacter.BP_FirstPersonCharacter_C|GetPlayer%20Movement%20History _player_ref_2))
  (bind _player_starting_location (Variables|/Game/FirstPerson/Blueprints/BP_FirstPersonCharacter.BP_FirstPersonCharacter_C|GetPlayer%20Starting%20Location _player_ref))
  (if (not (Variables|Default|GetTimer%20Started?))
    (bind _returnvalue (Game|SpawnActorfromClass "/Game/Blueprints/BP_Target.BP_Target_C" (Math|Conversions|ToTransform(Vector) _player_starting_location) "Undefined" "MultiplyWithRoot" 0 0))
    (Transformation|SetWorldLocation (Variables|/Game/Blueprints/BP_Target.BP_Target_C|GetCube _returnvalue) (Math|Vector|Lerp(Vector) _player_starting_location (Utilities|Array|Get(acopy) _player_movement_history (- (Utilities|Array|Length _player_movement_history) 1)) 0.0) false false)))

(event Custom|Count%20Targets
  ;[0.15 0.15 0.15 0.5] From 3D Tutorial
  (bind _outactors (Actor|GetAllActorsOfClass "/Game/Blueprints/BP_Target.BP_Target_C"))
  (Variables|Default|SetTargets (Utilities|Array|Length _outactors)))

(event Custom|Round%20Over
  (bind _returnvalue (Game|GetPlayerController 0))
  ;[0.15 0.15 0.15 0.5] From 3D Tutorial
  (Variables|Default|SetTimer%20Started? false)
  (Utilities|FlowControl|Delay 1.0)
  (Game|SetGamePaused true)
  (Variables|/Script/Engine.PlayerController|SetbShowMouseCursor _returnvalue true)
  (Input|SetInputModeUIOnly _returnvalue 0 "DoNotLock" false)
  (bind _asbp_first_person_character (Utilities|Casting|CastToBP_FirstPersonCharacter (Game|GetPlayerCharacter 0)))
  (Default|ShowNextRound (Variables|/Game/FirstPerson/Blueprints/BP_FirstPersonCharacter.BP_FirstPersonCharacter_C|GetUI%20Ref _asbp_first_person_character))
  (CallFunction|NextRound))

(event Custom|Target%20Hit?
  ;[0.15 0.15 0.15 0.5] From 3D Tutorial
  (if (Variables|Default|GetTimer%20Started?)
    (Math|Integer|DecrementInt (Variables|Default|GetTargets)
      (:%20%20
        (CallFunction|CheckifRoundOver)))))

(event Custom|Decrement%20Timer
  (params (Time%20Passed :type Float%20%28double-precision%29))
  ;[0.15 0.15 0.15 0.5] Reworked Increment Timer into a Decrement Timer from 3D Tutorial
  (bind _output_get (Variables|Default|SetTotal%20Time (- (Variables|Default|GetTotal%20Time) Time%20Passed)))
  (Variables|Default|SetRounded%20Time (Utilities|String|ToString(Integer) (Math|Float|Round _output_get)))
  (CallFunction|CheckifGameOver))

(event Custom|Check%20if%20Round%20Over
  (if (== (Variables|Default|GetTargets) 0)
    (CallFunction|RoundOver)
    (CallFunction|CreateNewTarget)))

(event Custom|Next%20Round
  (bind _returnvalue (Game|GetPlayerController 0))
  (CallFunction|Start)
  (Game|SetGamePaused false)
  (Variables|/Script/Engine.PlayerController|SetbShowMouseCursor _returnvalue false)
  (Input|SetInputModeGameOnly _returnvalue false)
  (Math|Integer|IncrementInt (Variables|Default|GetRound%20Number)
    (:%20%20
      (CallFunction|CountTargets)
      (CallFunction|Countdown))))

(event Custom|Countdown
  (Variables|Default|SetTotal%20Time (Math|Conversions|ToFloat(Integer) (* (Variables|Default|GetTargets) (Variables|Default|GetTarget%20Time)))))

(event Custom|Game%20Over
  (bind _returnvalue (Game|GetPlayerController 0))
  ;[0.15 0.15 0.15 0.5] From 3D Tutorial
  (Variables|Default|SetTimer%20Started? false)
  (Utilities|FlowControl|Delay 1.0)
  (Game|SetGamePaused true)
  (Variables|/Script/Engine.PlayerController|SetbShowMouseCursor _returnvalue true)
  (Input|SetInputModeUIOnly _returnvalue 0 "DoNotLock" false)
  (bind _asbp_first_person_character (Utilities|Casting|CastToBP_FirstPersonCharacter (Game|GetPlayerCharacter 0)))
  (Default|ShowGameOver (Variables|/Game/FirstPerson/Blueprints/BP_FirstPersonCharacter.BP_FirstPersonCharacter_C|GetUI%20Ref _asbp_first_person_character)))

(event EventTick
  (params (DeltaSeconds :type Float%20%28single-precision%29))
  (if (Variables|Default|GetTimer%20Started?)
    (if (not (<= (Variables|Default|GetTotal%20Time) 0.0))
      (CallFunction|DecrementTimer (* DeltaSeconds 2.0)))))

(event EventBeginPlay
  ;[0.15 0.15 0.15 0.5] From 3D Tutorial
  (CallFunction|CountTargets)
  (CallFunction|Countdown)
  (Game|SetGamePaused false)
  (Input|SetInputModeGameOnly (Game|GetPlayerController 0) false)
  (bind _asbp_first_person_character (Utilities|Casting|CastToBP_FirstPersonCharacter (Game|GetPlayerCharacter 0)))
  (bind _output_get (Variables|Default|SetPlayer%20Ref _asbp_first_person_character))
  (Utilities|FlowControl|DoOnce false
    (:Completed
      (Default|PlayerStart _output_get))))

(fn ConstructionScript)